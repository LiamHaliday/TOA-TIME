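; A player controller that lets the player switch possession between a vehicle pawn and the third-person character.
; Keys 1 and 2 possess the first VehicleBlueprint and first ThirdPersonCharacter found by class lookup.
; Key E picks either target from the BoatView flag, which only key H toggles, so possessing a pawn leaves the flag unchanged.
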(event EventBeginPlay)

(event Input|KeyboardEvents|2
  (params (Key :type Key%20Structure :default "AnyKey"))
  (:Pressed
    (bind _outactors (Actor|GetAllActorsOfClass "/Game/ThirdPersonBP/Blueprints/ThirdPersonCharacter.ThirdPersonCharacter_C"))
    (Pawn|Possess (Utilities|Array|Get(acopy) _outactors))))

(event Input|KeyboardEvents|E
  (params (Key :type Key%20Structure :default "AnyKey"))
  (:Pressed
    (if (Variables|Default|GetboatView) ; Only on first touch
      (bind _outactors (Actor|GetAllActorsOfClass "/Game/VehicleAdvBP/Blueprints/VehicleBlueprint.VehicleBlueprint_C"))
      (Pawn|Possess (Utilities|Array|Get(acopy) _outactors))
      (else
        (bind _outactors_2 (Actor|GetAllActorsOfClass "/Game/ThirdPersonBP/Blueprints/ThirdPersonCharacter.ThirdPersonCharacter_C"))
        (Pawn|Possess (Utilities|Array|Get(acopy) _outactors_2))))))

(event Input|KeyboardEvents|1
  (params (Key :type Key%20Structure :default "AnyKey"))
  (:Pressed
    (bind _outactors (Actor|GetAllActorsOfClass "/Game/VehicleAdvBP/Blueprints/VehicleBlueprint.VehicleBlueprint_C"))
    (Pawn|Possess (Utilities|Array|Get(acopy) _outactors))))

(event Input|KeyboardEvents|H
  (params (Key :type Key%20Structure :default "AnyKey"))
  (:Pressed
    (Variables|Default|SetboatView (not (Variables|Default|GetboatView)))))

(fn ConstructionScript)